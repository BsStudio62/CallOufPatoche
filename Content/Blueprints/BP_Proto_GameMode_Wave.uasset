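; Prototype wave-mode GameMode that initializes zombie spawning and wave state when play begins.
; If a spawner manager exists, BeginPlay passes it the zombie activation setting, collects all spawn points as possible spawns, and sets wave 1 on the GameState, firing its change notification.
; Player spawning, distance-based spawn point filtering with color feedback and debug drawing are present but disconnected, and the other events are empty.
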(event EventOnLogout
  (params (ExitingController :type Controller%20Object%20Reference)))

(event EventPostLogin
  (params (NewPlayer :type Player%20Controller%20Object%20Reference)))

(event EventBeginPlay
  (bind _returnvalue (Actor|GetActorOfClass "/Game/Blueprints/Spawner/BP_SpawnerManager.BP_SpawnerManager_C"))
  (Utilities|IsValid _returnvalue
    (:Is%20Valid
      (Variables|/Game/Blueprints/Spawner/BP_SpawnerManager.BP_SpawnerManager_C|SetbActivatedZombie _returnvalue (Variables|Default|GetActivated%20Zombie))
      ;[1 1 1] Spawn Points Zombie
      (bind _outactors (Actor|GetAllActorsOfClass "/Game/Blueprints/Spawner/BP_SpawnerPoint.BP_SpawnerPoint_C"))
      (bind _output_get (Variables|Default|SetSpawnerPoints _outactors))
      (Variables|Default|SetSpawnPointPossible _output_get)
      (bind _asbp_proto_game_state_wave (Utilities|Casting|CastToBP_Proto_GameState_Wave (Game|GetGameState)))
      (Variables|Default|SetAs%20BP%20Proto%20Game%20State%20Wave _asbp_proto_game_state_wave)
      (bind _output_get_2 (Variables|Default|SetWaves 1))
      (Variables|/Game/Blueprints/BP_Proto_GameState_Wave.BP_Proto_GameState_Wave_C|SetWave (Variables|Default|GetAs%20BP%20Proto%20Game%20State%20Wave) _output_get_2)
      (Default|CallOnChangeWaves (Variables|Default|GetAs%20BP%20Proto%20Game%20State%20Wave)))))

(event EventTick
  (params (DeltaSeconds :type Float%20%28single-precision%29)))

(fn ConstructionScript)