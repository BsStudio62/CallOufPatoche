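; BP_WallWindows is a Geometry Scripting tool that procedurally generates a wall with a box-shaped window opening.
; On mesh rebuild, it appends a wall box sized by Cursor and offset by half its X and Y size.
; A second box, placed by PositionWindows and sized by CursorWindows, is built in a temporary compute mesh.
; A boolean subtract cuts that box from the wall, filling holes and simplifying output, then compute meshes are released.
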(event Events|EventOnRebuildGeneratedMesh
  (params (TargetMesh :type Dynamic%20Mesh%20Object%20Reference))
  (bind _cursorwindows (Variables|Default|GetCursorWindows))
  (bind _cursor (Variables|Default|GetCursor))
  (bind _cursor_2 (Variables|Default|GetCursor))
  (bind _positionwindows (Variables|Default|GetPositionWindows))
  (bind (_x _y _z) (Math|Vector|BreakVector _cursorwindows))
  (bind (_x_2 _y_2 _z_2) (Math|Vector|BreakVector _positionwindows))
  (bind (_x_3 _y_3 _z_3) (Math|Vector|BreakVector _cursor))
  (bind (_x_4 _y_4) (Math|Vector|BreakVector _cursor_2))
  (bind _returnvalue (Class|GeometryScriptLibraryMeshPrimitiveFunctions|AppendBox :TargetMesh TargetMesh :Transform (Math|Transform|MakeTransform (Math|Vector|MakeVector (/ _x_4 2.0) (/ _y_4 2.0) 0.0) "0, 0, 0" "1.000000,1.000000,1.000000") :DimensionX _x_3 :DimensionY _y_3 :DimensionZ _z_3 :Debug 0))
  (bind _returnvalue_2 (DynamicMeshActor|AllocateComputeMesh))
  (bind _returnvalue_3 (Class|GeometryScriptLibraryMeshPrimitiveFunctions|AppendBox :TargetMesh _returnvalue_2 :Transform (Math|Transform|MakeTransform (Math|Vector|MakeVector _x_2 _y_2 _z_2) "0, 0, 0" "1.000000,1.000000,1.000000") :DimensionX _x :DimensionY _y :DimensionZ _z :Debug 0))
  (GeometryScript|Booleans|ApplyMeshBoolean :TargetMesh _returnvalue :ToolMesh _returnvalue_3 :Operation "Subtract" :Options (Utilities|Struct|MakeGeometryScriptMeshBooleanOptions true true 0.01) :Debug 0)
  (DynamicMeshActor|ReleaseAllComputeMeshes))

(fn ConstructionScript
  (|CallParentFunction))