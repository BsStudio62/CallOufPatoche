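; Geometry Scripting wall tool actor that generates a simple box mesh, named as the no-collision wall variant.
; On mesh rebuild it appends a box sized by the Cursor vector, offset by half its X and Y so it extends from the actor origin.
; It then releases the compute meshes and sets the DynamicMeshComponent visibility.
; The construction script only calls the parent, and no collision setup appears in the graphs.
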(event Events|EventOnRebuildGeneratedMesh
  (params (TargetMesh :type Dynamic%20Mesh%20Object%20Reference))
  (bind _cursor (Variables|Default|GetCursor))
  (bind _cursor_2 (Variables|Default|GetCursor))
  (bind (_x _y _z) (Math|Vector|BreakVector _cursor))
  (bind (_x_2 _y_2) (Math|Vector|BreakVector _cursor_2))
  (Class|GeometryScriptLibraryMeshPrimitiveFunctions|AppendBox :TargetMesh TargetMesh :Transform (Math|Transform|MakeTransform (Math|Vector|MakeVector (/ _x_2 2.0) (/ _y_2 2.0) 0.0) "0, 0, 0" "1.000000,1.000000,1.000000") :DimensionX _x :DimensionY _y :DimensionZ _z :Debug 0)
  (DynamicMeshActor|ReleaseAllComputeMeshes)
  (Rendering|SetVisibility (Variables|Default|GetDynamicMeshComponent) (Variables|Default|GetNew%20Visibility) false))

(fn ConstructionScript
  (|CallParentFunction))