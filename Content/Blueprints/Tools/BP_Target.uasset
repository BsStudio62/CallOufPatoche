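; BP_Target is a tool actor that shows the distance between a Start and an End point as a label in metres.
; Its construction script takes the absolute X difference divided by 100, writes it to a TextRender with a "Mètre" suffix, and moves the SkeletalMesh to End.
; Only the X axis counts, and the event graph holds no active logic.
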(event EventBeginPlay)

(event Collision|EventActorBeginOverlap
  (params (OtherActor :type Actor%20Object%20Reference)))

(event EventTick
  (params (DeltaSeconds :type Float%20%28single-precision%29)))

(fn ConstructionScript
  (bind _output_get (Variables|Default|SetDistance (/ (Math|Float|Absolute(Float) (- (.x (Variables|Default|GetStart)) (.x (Variables|Default|GetEnd)))) 1e+02)))
  (Rendering|Components|TextRender|SetText (Variables|Default|GetTextRender) (Utilities|Text|FormatText "{float} Mètre" _output_get))
  (Transformation|SetRelativeLocation (Variables|Default|GetSkeletalMesh) (Variables|Default|GetEnd) false false))