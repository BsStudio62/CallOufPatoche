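; BP_Target is a target character that reacts to taking damage.
; On any damage event it hides the "head" bone of its skeletal mesh, waits five seconds, then unhides it.
; Logic for awarding points to the player state and refreshing the first-person controller's widget is present but unconnected, so it never runs.
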(event EventDamage
  (params (Damage :type Float%20%28double-precision%29))
  (Components|SkinnedMesh|HideBonebyName (Variables|Default|GetSkeletalMesh) "head" "PBO_None")
  (Utilities|FlowControl|Delay 5.0)
  (Components|SkinnedMesh|UnHideBonebyName (Variables|Default|GetSkeletalMesh) "head"))

(fn ConstructionScript)