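; BP_GameMode_Wave is a wave game mode that tracks which spawner points are near players, without spawning anything itself.
; It records controllers at PostLogin, then gathers their pawns and all BP_SpawnerPoint actors once at BeginPlay.
; Every Tick, it tests each point against each pawn's distance, coloring it green and adding it to SpawnPointPossible, or red and removing it.
; The last pawn checked decides each point's state.
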(event EventPostLogin
  (params (NewPlayer :type Player%20Controller%20Object%20Reference))
  (Utilities|Array|AddUnique (Variables|Default|GetPlayerControllers) NewPlayer))

(event EventBeginPlay
  (bind _outactors (Actor|GetAllActorsOfClass "/Game/Blueprints/Spawner/BP_SpawnerPoint.BP_SpawnerPoint_C"))
  (Variables|Default|SetSpawnerPoints _outactors)
  (for _array_element (Variables|Default|GetPlayerControllers)
    (Utilities|Array|AddUnique (Variables|Default|GetPlayerPawns) (Pawn|GetControlledPawn _array_element))))

(event EventTick
  (params (DeltaSeconds :type Float%20%28single-precision%29))
  (bind _spawnpointpossible (Variables|Default|GetSpawnPointPossible))
  (if (Utilities|Array|IsValidIndex (Variables|Default|GetSpawnerPoints))
    (for _array_element (Variables|Default|GetSpawnerPoints)
      (for _array_element_2 (Variables|Default|GetPlayerPawns)
        (if (< (Transformation|GetDistanceTo _array_element _array_element_2) (Variables|Default|GetDistance))
          (Default|SetColor _array_element "(R=0.000000,G=1.000000,B=0.107579,A=1.000000)")
          (Utilities|Array|AddUnique _spawnpointpossible _array_element)
          (else
            (Default|SetColor _array_element "(R=1.000000,G=0.000000,B=0.000000,A=1.000000)")
            (Utilities|Array|RemoveItem _spawnpointpossible _array_element)))))))

(fn ConstructionScript)