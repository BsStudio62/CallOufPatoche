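; Prototype zombie teleporter that sends characters entering its Box to the Teleportation component's transform once the linked RefBarricade is open.
; On server overlap, it teleports immediately if open; otherwise it enables Tick to poll the barricade.
; When the barricade opens, Tick teleports all overlapping characters, then disables itself.
; Teleported actors have AI movement stopped, and BP_Zombies are ordered to follow player 0.
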(event OnComponentBeginOverlap(Box)
  (params (OverlappedComponent :type Primitive%20Component%20Object%20Reference) (OtherActor :type Actor%20Object%20Reference) (OtherComp :type Primitive%20Component%20Object%20Reference) (OtherBodyIndex :type Integer) (bFromSweep :type Boolean) (SweepResult :type Hit%20Result%20Structure%20%28by%20ref%29))
  (bind _teleportation (Variables|Default|GetTeleportation))
  (bind _returnvalue (Transformation|GetWorldTransform _teleportation))
  (Networking|SwitchHasAuthority
    (:Authority
      (bind _refbarricade (Variables|Default|GetRefBarricade)
        (:then
          (if (Variables|/Game/Blueprints/Barricade/BP_Barricade.BP_Barricade_C|GetbIsOpen _refbarricade)
            (Transformation|Teleport OtherActor (.location _returnvalue) (.rotation _returnvalue))
            (AI|Navigation|StopMovement (AI|GetAIController OtherActor))
            (bind _asbp_zombie (Utilities|Casting|CastToBP_Zombie OtherActor))
            ;[1 1 1] Follow Player
            (Default|Move _asbp_zombie "0, 0, 0" (Game|GetPlayerCharacter 0) "NewEnumerator0")
            (else
              (Actor|Tick|SetActorTickEnabled true))))
        (:else)))))

(event EventTick
  (params (DeltaSeconds :type Float%20%28single-precision%29))
  (bind _teleportation (Variables|Default|GetTeleportation))
  (bind _returnvalue (Transformation|GetWorldTransform _teleportation))
  (bind _refbarricade (Variables|Default|GetRefBarricade)
    (:then
      (if (Variables|/Game/Blueprints/Barricade/BP_Barricade.BP_Barricade_C|GetbIsOpen _refbarricade)
        (for _array_element (Collision|GetOverlappingActors (Variables|Default|GetBox) "/Script/Engine.Character" :!class /Script/Engine.PrimitiveComponent)
          (Transformation|Teleport _array_element (.location _returnvalue) (.rotation _returnvalue))
          (AI|Navigation|StopMovement (AI|GetAIController _array_element))
          (bind _asbp_zombie (Utilities|Casting|CastToBP_Zombie _array_element))
          ;[1 1 1] Follow Player
          (Default|Move _asbp_zombie "0, 0, 0" (Game|GetPlayerCharacter 0) "NewEnumerator0"))
        (Actor|Tick|SetActorTickEnabled false)))
    (:else)))

(fn ConstructionScript)