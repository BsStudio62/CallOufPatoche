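; Zombie enemy that chases the player, breaks through barricades and can drop loot when destroyed.
; An enum action state checked on Tick, with the InBuilding flag and barricade state, picks between AI MoveTo on the player, which deals damage on arrival, and on a closed barricade.
; At a barricade, a looping timer plays a montage and removes pieces until it opens.
; On destruction it rolls against DT_Drops and removes itself from its spawner.
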(event Custom|Move
  (params (Destination :type Vector) (TargetActor :type Actor%20Object%20Reference) (Zombie%20Action :type E_ZombieAction%20Enum :default "NewEnumerator0"))
  (Variables|Default|SetZombieAction Zombie%20Action)
  (bind _asbp_proto_player (Utilities|Casting|CastToBP_Proto_Player TargetActor)
    (:then
      ;[1 1 1] Damage
      (AI|AIMoveTo self "0, 0, 0" TargetActor 5.0 false
        (:OnSuccess
          (Default|CallOnHealthDamaged (Variables|/Game/Blueprints/Characters/Proto/BP_Proto_Player.BP_Proto_Player_C|GetBP_Stats _asbp_proto_player) 25.0 "SurfaceType_Default"))))
    (:CastFailed
      (bind _movementresult (AI|AIMoveTo self Destination TargetActor 5.0 false)
        (:then
          (bind _asbp_barricade (Utilities|Casting|CastToBP_Barricade TargetActor))
          (Variables|Default|SetAs%20BP%20Barricade _asbp_barricade))
        (:OnSuccess
          (Development|PrintString "Sucess")
          (Variables|Default|SetZombieAction "NewEnumerator3"))
        (:OnFail
          (Development|PrintString (Utilities|String|EnumtoString _movementresult)))))))

(event Custom|Destroy%20Windows
  (bind _asbp_barricade (Utilities|Casting|CastToBP_Barricade (Variables|Default|GetOtherActor)))
  (bind _output_get (Variables|Default|SetAs%20BP%20Barricade _asbp_barricade))
  (if (Variables|/Game/Blueprints/Barricade/BP_Barricade.BP_Barricade_C|GetbIsOpen _output_get)
    (Utilities|Time|ClearandInvalidateTimerbyHandle (Variables|Default|GethandleDestroyWindows))
    (CallFunction|Move "0, 0, 0" (Game|GetPlayerCharacter 0) "NewEnumerator3")
    (else
      (Animation|Montage|PlayMontage (Variables|Character|GetMesh) 0
        (:then
          (Default|RemoveBarricade (Variables|Default|GetAs%20BP%20Barricade)))))))

(event Custom|Activate%20Timer
  (bind _returnvalue (Utilities|Time|SetTimerbyEvent (delegate Custom|Destroy%20Windows) 2.0 true))
  (Variables|Default|SethandleDestroyWindows _returnvalue))

(event Custom|Move%20Barricade
  (params (Destination :type Vector) (Barricade :type BP%20Barricade%20Object%20Reference) (ZombieAction :type E_ZombieAction%20Enum :default "NewEnumerator0"))
  ;[1 1 1] Move to Barricade
  (Variables|Default|SetZombieAction ZombieAction)
  (Variables|Default|SetOtherActor Barricade)
  (AI|AIMoveTo self Destination 0 5.0 false
    (:OnSuccess
      (CallFunction|ActivateTimer))
    (:OnFail
      (Variables|Default|SetZombieAction "NewEnumerator3")
      (Development|PrintString "Fail BArricade"))))

(event EventTick
  (params (DeltaSeconds :type Float%20%28single-precision%29))
  (bind _as_bp_barricade (Variables|Default|GetAs%20BP%20Barricade))
  (if (Variables|Default|GetInBuilding)
    (if (Utilities|Enum|Equal(Enum) (Variables|Default|GetZombieAction) "NewEnumerator3") :!label _label
      (CallFunction|Move "0, 0, 0" (Game|GetPlayerCharacter 0) "NewEnumerator2"))
    (else
      (bind _as_bp_barricade_2 (Variables|Default|GetAs%20BP%20Barricade)
        (:then
          (if (Variables|/Game/Blueprints/Barricade/BP_Barricade.BP_Barricade_C|GetbIsOpen _as_bp_barricade_2)
            (goto _label)
            (elif (Utilities|Enum|Equal(Enum) (Variables|Default|GetZombieAction) "NewEnumerator2")
              (CallFunction|MoveBarricade (Transformation|GetActorLocation _as_bp_barricade) _as_bp_barricade "NewEnumerator1")
              (elif (Utilities|Enum|Equal(Enum) (Variables|Default|GetZombieAction) "NewEnumerator3")
                _))))
        (:else)))))

(event EventBeginPlay
  (CallFunction|Move "0, 0, 0" (Game|GetPlayerCharacter 0) "NewEnumerator2"))

(event EventDamage
  (params (Damage :type Float%20%28double-precision%29))
  (Default|CallOnHealthDamaged (Variables|Default|GetBP_Stats) 1e+01 "SurfaceType_Default"))

(event EventDestroyed
  ;[1 1 1] Drops
  (Variables|Default|SetDrops (Math|Random|RandomFloatinRange 0.0 1e+02))
  (bind _outrownames (DataTable|GetDataTableRowNames "/Game/Blueprints/DataTable/DT_Drops.DT_Drops"))
  (bind _array_element (Utilities|Array|ForEachLoopwithBreak _outrownames :!label _label)
    (:LoopBody
      (bind _returnvalue (Utilities|GetDataTableRow "/Game/Blueprints/DataTable/DT_Drops.DT_Drops" _array_element)
        (:then
          (if (<= (Variables|Default|GetDrops) (.Drop (Utilities|Struct|BreakSDropItem _returnvalue)))
            (Variables|Default|SetOut%20Row _returnvalue)
            (Variables|Default|SetNoDrops false)
            (goto _label Break)))))
    (:Completed
      (if (Variables|Default|GetNoDrops)
        _
        (else
          (Game|SpawnActorfromClass (Utilities|Struct|BreakSDropItem (Variables|Default|GetOut%20Row)) (Math|Transform|MakeTransform (Transformation|GetActorLocation) "0, 0, 0" "1.000000,1.000000,1.000000") "AlwaysSpawn" "MultiplyWithRoot" 0 0)))
      (bind _spawner (Variables|Default|GetSpawner)
        (:then
          (Default|RemoveZombies _spawner self))
        (:else)))))

(fn ConstructionScript)