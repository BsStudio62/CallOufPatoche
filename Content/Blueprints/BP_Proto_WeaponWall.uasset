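; BP_Proto_WeaponWall is a prototype interactable wall point that sells an ammo refill for the player's current weapon.
; A sphere overlap registers it as the player's interaction and shows a priced prompt through the player controller, clearing both on exit.
; Interact skips full weapons, checks the PlayerState score against a hard-coded cost, then deducts it, refills munition and calls the weapon's fire update.
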(event OnComponentBeginOverlap(Sphere)
  (params (OverlappedComponent :type Primitive%20Component%20Object%20Reference) (OtherActor :type Actor%20Object%20Reference) (OtherComp :type Primitive%20Component%20Object%20Reference) (OtherBodyIndex :type Integer) (bFromSweep :type Boolean) (SweepResult :type Hit%20Result%20Structure%20%28by%20ref%29))
  (bind _asbp_player (Utilities|Casting|CastToBP_Player OtherActor))
  (Variables|/Game/Blueprints/BP_Player.BP_Player_C|SetInteraction _asbp_player self)
  (bind _asbp_first_person_player_controller (Utilities|Casting|CastToBP_FirstPersonPlayerController (Game|GetInstigatorController _asbp_player)))
  (Default|SetInteraction _asbp_first_person_player_controller "Munition" "100")
  (Default|SetActive&DisableInteraction _asbp_first_person_player_controller "Visible"))

(event OnComponentEndOverlap(Sphere)
  (params (OverlappedComponent :type Primitive%20Component%20Object%20Reference) (OtherActor :type Actor%20Object%20Reference) (OtherComp :type Primitive%20Component%20Object%20Reference) (OtherBodyIndex :type Integer))
  (bind _asbp_player (Utilities|Casting|CastToBP_Player OtherActor))
  (Variables|/Game/Blueprints/BP_Player.BP_Player_C|SetInteraction _asbp_player 0)
  (bind _asbp_first_person_player_controller (Utilities|Casting|CastToBP_FirstPersonPlayerController (Game|GetInstigatorController _asbp_player)))
  (Default|SetActive&DisableInteraction _asbp_first_person_player_controller "Hidden"))

(event EventInteract
  (params (Player :type BP%20Player%20Object%20Reference))
  (bind _weapon (Variables|/Game/Blueprints/BP_Player.BP_Player_C|GetWeapon Player))
  (bind _full (Default|CheckFullMunition (Variables|/Game/Blueprints/BP_Player.BP_Player_C|GetWeapon Player)))
  (if (not _full)
    (bind _asbp_proto_player_state (Utilities|Casting|CastToBP_Proto_PlayerState (Variables|/Script/Engine.Controller|GetPlayerState (Game|GetInstigatorController Player))))
    (if (> (Variables|/Game/Blueprints/BP_Proto_PlayerState.BP_Proto_PlayerState_C|GetScoreProto _asbp_proto_player_state) 1e+02)
      (Default|SetScore _asbp_proto_player_state -1e+02)
      (Default|RefillMunition _weapon)
      (Default|CallOnFireUpdate _weapon))))

(fn ConstructionScript)

(fn GetInteractable
  (return "NewEnumerator1"))

(fn GetPossibleInteraction
  (return false))