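; Prototype purchasable door that disappears when a player with enough score interacts with it.
; A box overlap registers the door as the player's current Interaction and has the player controller show a prompt with text and price, clearing both on exit.
; Interact compares PlayerState score to Cost, updates the score, hides the prompt and destroys the door.
; Interaction getters return a fixed type and false for possible interaction.
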(event OnComponentBeginOverlap(Box)
  (params (OverlappedComponent :type Primitive%20Component%20Object%20Reference) (OtherActor :type Actor%20Object%20Reference) (OtherComp :type Primitive%20Component%20Object%20Reference) (OtherBodyIndex :type Integer) (bFromSweep :type Boolean) (SweepResult :type Hit%20Result%20Structure%20%28by%20ref%29))
  (bind _asbp_player (Utilities|Casting|CastToBP_Proto_Player OtherActor))
  (Variables|/Game/Blueprints/Characters/Proto/BP_Proto_Player.BP_Proto_Player_C|SetInteraction _asbp_player self)
  (bind _asbp_first_person_player_controller (Utilities|Casting|CastToBP_FirstPersonPlayerController (Game|GetInstigatorController _asbp_player)))
  (Default|SetInteraction _asbp_first_person_player_controller (Variables|Default|GetText%20Interaction) (Utilities|Text|ToText(Float) (Variables|Default|GetCost) "HalfToEven"))
  (Default|SetActive&DisableInteraction _asbp_first_person_player_controller "Visible"))

(event OnComponentEndOverlap(Box)
  (params (OverlappedComponent :type Primitive%20Component%20Object%20Reference) (OtherActor :type Actor%20Object%20Reference) (OtherComp :type Primitive%20Component%20Object%20Reference) (OtherBodyIndex :type Integer))
  (bind _asbp_player (Utilities|Casting|CastToBP_Proto_Player OtherActor))
  (Variables|/Game/Blueprints/Characters/Proto/BP_Proto_Player.BP_Proto_Player_C|SetInteraction _asbp_player 0)
  (bind _asbp_first_person_player_controller (Utilities|Casting|CastToBP_FirstPersonPlayerController (Game|GetInstigatorController _asbp_player)))
  (Default|SetActive&DisableInteraction _asbp_first_person_player_controller "Hidden"))

(event EventInteract
  (params (Player :type BP%20Proto%20Player%20Object%20Reference))
  (bind _asbp_first_person_player_controller (Utilities|Casting|CastToBP_FirstPersonPlayerController (Game|GetInstigatorController Player)))
  (bind _asbp_proto_player_state (Utilities|Casting|CastToBP_Proto_PlayerState (Variables|/Script/Engine.Controller|GetPlayerState _asbp_first_person_player_controller)))
  (if (>= (Variables|/Game/Blueprints/BP_Proto_PlayerState.BP_Proto_PlayerState_C|GetScoreProto _asbp_proto_player_state) (Variables|Default|GetCost))
    (bind _result (Math|Float|NegateFloat (Variables|Default|GetCost))
      (:%20%20
        (Default|SetScore _asbp_proto_player_state _result)
        (Default|SetActive&DisableInteraction _asbp_first_person_player_controller "Hidden")
        (Actor|DestroyActor)))))

(fn ConstructionScript)

(fn GetInteractable
  (return "NewEnumerator1"))

(fn GetPossibleInteraction
  (return false))