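; Master wall-weapon interactable that lets the player buy a weapon or refill its ammo.
; Sphere overlap picks refill if the weapon is equipped or buy if not owned, registers as the player's interaction and shows a HUD prompt with price.
; Interact either refills non-full ammo against player score, or replaces the current weapon and updates the HUD, with no score check.
; The construction script applies the configured mesh and material.
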(event OnComponentBeginOverlap(Sphere)
  (params (OverlappedComponent :type Primitive%20Component%20Object%20Reference) (OtherActor :type Actor%20Object%20Reference) (OtherComp :type Primitive%20Component%20Object%20Reference) (OtherBodyIndex :type Integer) (bFromSweep :type Boolean) (SweepResult :type Hit%20Result%20Structure%20%28by%20ref%29))
  (bind _asbp_proto_player (Utilities|Casting|CastToBP_Proto_Player OtherActor))
  (bind _output_get (Variables|Default|SetAs%20BP%20Player _asbp_proto_player))
  (bind _bisexist (Default|CheckWeaponExistinInventory _output_get (Variables|Default|GetNameWeapon)))
  (if _bisexist
    (bind _bisequiped (Default|CheckWeaponEquiped (Variables|Default|GetAs%20BP%20Player) (Variables|Default|GetNameWeapon)))
    (if _bisequiped
      (Variables|Default|SetActions "NewEnumerator0")
      (Variables|/Game/Blueprints/Characters/Proto/BP_Proto_Player.BP_Proto_Player_C|SetInteraction (Variables|Default|GetAs%20BP%20Player) self :!label _label)
      (bind _asbp_first_person_player_controller (Utilities|Casting|CastToBP_FirstPersonPlayerController (Game|GetInstigatorController (Variables|Default|GetAs%20BP%20Player))))
      (Default|SetInteraction _asbp_first_person_player_controller (Utilities|Select :Index (Variables|Default|GetActions) :NewEnumerator0 "Munition" :NewEnumerator1 (Utilities|Text|FormatText "By {Weapon}" (Variables|Default|GetNameWeapon))) (Utilities|Text|ToText(Float) (Variables|Default|GetCost) "HalfToEven" false true 1 324 0 0))
      (Default|SetActive&DisableInteraction _asbp_first_person_player_controller "Visible"))
    (else
      (Variables|Default|SetActions "NewEnumerator1")
      (goto _label))))

(event OnComponentEndOverlap(Sphere)
  (params (OverlappedComponent :type Primitive%20Component%20Object%20Reference) (OtherActor :type Actor%20Object%20Reference) (OtherComp :type Primitive%20Component%20Object%20Reference) (OtherBodyIndex :type Integer))
  (bind _asbp_proto_player (Utilities|Casting|CastToBP_Proto_Player OtherActor))
  (Variables|/Game/Blueprints/Characters/Proto/BP_Proto_Player.BP_Proto_Player_C|SetInteraction _asbp_proto_player 0)
  (bind _asbp_first_person_player_controller (Utilities|Casting|CastToBP_FirstPersonPlayerController (Game|GetInstigatorController _asbp_proto_player)))
  (Default|SetActive&DisableInteraction _asbp_first_person_player_controller "Hidden"))

(event EventInteract
  (params (Player :type BP%20Proto%20Player%20Object%20Reference))
  (bind _currentweapon (Variables|/Game/Blueprints/Characters/Proto/BP_Proto_Player.BP_Proto_Player_C|GetCurrentWeapon Player))
  (switch Utilities|FlowControl|Switch|SwitchonE_Action (Variables|Default|GetActions)
    (:NewEnumerator0
      (bind _full (Default|CheckFullMunition (Variables|/Game/Blueprints/Characters/Proto/BP_Proto_Player.BP_Proto_Player_C|GetCurrentWeapon Player)))
      (if (not _full)
        (bind _asbp_proto_player_state (Utilities|Casting|CastToBP_Proto_PlayerState (Variables|/Script/Engine.Controller|GetPlayerState (Game|GetInstigatorController Player))))
        (if (> (Variables|/Game/Blueprints/BP_Proto_PlayerState.BP_Proto_PlayerState_C|GetScoreProto _asbp_proto_player_state) (Variables|Default|GetCost))
          (bind _result (Math|Float|NegateFloat (Variables|Default|GetCost))
            (:%20%20
              (Default|SetScore _asbp_proto_player_state _result)
              (Default|RefillMunition _currentweapon)
              (Default|CallOnFireUpdate _currentweapon))))))
    (:NewEnumerator1
      (Actor|DestroyActor (Variables|/Game/Blueprints/Characters/Proto/BP_Proto_Player.BP_Proto_Player_C|GetCurrentWeapon Player))
      (Variables|/Game/Blueprints/Characters/Proto/BP_Proto_Player.BP_Proto_Player_C|SetWeaponStarterClass Player (Variables|Default|GetWeaponClass))
      (Default|SpawnWEapon Player)
      (Variables|/Game/Blueprints/Characters/Proto/BP_Proto_Player.BP_Proto_Player_C|SetSelectWeapon Player 1)
      (bind _asbp_first_person_player_controller (Utilities|Casting|CastToBP_FirstPersonPlayerController (Game|GetInstigatorController Player)))
      (Default|CallOnUpdateWeapon (Variables|/Game/Blueprints/Widget/WBP_Hud.WBP_Hud_C|GetWBP_Weapon (Variables|/Game/Blueprints/BP_FirstPersonPlayerController.BP_FirstPersonPlayerController_C|GetRefHud _asbp_first_person_player_controller))))))

(fn ConstructionScript
  (Components|SkeletalMesh|SetSkeletalMeshAsset (Variables|Default|GetSkeletalMesh) (Variables|Default|GetSkinWeapon))
  (Rendering|Material|SetMaterial (Variables|Default|GetSkeletalMesh) 0 (Variables|Default|GetMaterialWeapon)))

(fn GetInteractable
  (return "NewEnumerator1"))

(fn GetPossibleInteraction
  (return false))