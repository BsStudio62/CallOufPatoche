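; Prototype mystery weapon box that cycles randomly ordered weapon meshes when a player interacts with it.
; BeginPlay loads skins and classes from DT_BoxMystery; Interact shuffles them, starts a Timeline and enables Tick to step the displayed mesh.
; Box overlap registers it as the player's interaction and toggles a priced prompt.
; Score payment is unwired, and no weapon is granted.
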(event OnComponentBeginOverlap(Box)
  (params (OverlappedComponent :type Primitive%20Component%20Object%20Reference) (OtherActor :type Actor%20Object%20Reference) (OtherComp :type Primitive%20Component%20Object%20Reference) (OtherBodyIndex :type Integer) (bFromSweep :type Boolean) (SweepResult :type Hit%20Result%20Structure%20%28by%20ref%29))
  (bind _asbp_proto_player (Utilities|Casting|CastToBP_Proto_Player OtherActor))
  (Variables|/Game/Blueprints/Characters/Proto/BP_Proto_Player.BP_Proto_Player_C|SetInteraction _asbp_proto_player self)
  (bind _asbp_first_person_player_controller (Utilities|Casting|CastToBP_FirstPersonPlayerController (Game|GetInstigatorController _asbp_proto_player)))
  (Default|SetInteraction _asbp_first_person_player_controller (Variables|Default|GetText%20Interaction) (Utilities|Text|ToText(Float) (Variables|Default|GetCost) "HalfToEven"))
  (Default|SetActive&DisableInteraction _asbp_first_person_player_controller "Visible"))

(event OnComponentEndOverlap(Box)
  (params (OverlappedComponent :type Primitive%20Component%20Object%20Reference) (OtherActor :type Actor%20Object%20Reference) (OtherComp :type Primitive%20Component%20Object%20Reference) (OtherBodyIndex :type Integer))
  (bind _asbp_proto_player (Utilities|Casting|CastToBP_Proto_Player OtherActor))
  (Variables|/Game/Blueprints/Characters/Proto/BP_Proto_Player.BP_Proto_Player_C|SetInteraction _asbp_proto_player 0)
  (bind _asbp_first_person_player_controller (Utilities|Casting|CastToBP_FirstPersonPlayerController (Game|GetInstigatorController _asbp_proto_player)))
  (Default|SetActive&DisableInteraction _asbp_first_person_player_controller "Hidden"))

(event Custom|AnimationWeapon)

(event EventInteract
  (params (Player :type BP%20Proto%20Player%20Object%20Reference))
  (Utilities|Array|Shuffle (Variables|Default|GetWeaponBoxMystery))
  (Actor|Tick|SetActorTickEnabled true)
  (Components|Timeline|PlayfromStart (Variables|Default|GetTimeline)))

(event EventBeginPlay
  (bind _outrownames (DataTable|GetDataTableRowNames "/Game/Blueprints/DataTable/DT_BoxMystery.DT_BoxMystery"))
  (for (_array_element _array_index) _outrownames
    (bind _returnvalue (Utilities|GetDataTableRow "/Game/Blueprints/DataTable/DT_BoxMystery.DT_BoxMystery" _array_element)
      (:then
        (Utilities|Array|SetArrayElem (Variables|Default|GetWeaponBoxMystery) _array_index (Utilities|Struct|MakeSBoxMystery (.weaponskin _returnvalue) (.class _returnvalue)) true)))))

(event EventTick
  (params (DeltaSeconds :type Float%20%28single-precision%29))
  (Components|Timeline|SetPlayRate (Variables|Default|GetTimeline) (/ 1.0 (Variables|Default|GetNew%20Rate)))
  (if (== (- (Utilities|Array|Length (Variables|Default|GetWeaponBoxMystery)) 1) (Variables|Default|GetIndex))
    (Variables|Default|SetIndex 0)
    (else
      (Math|Integer|IncrementInt (Variables|Default|GetIndex)
        (:%20%20
          _))))
  (Components|SkeletalMesh|SetSkeletalMeshAsset (Variables|Default|GetSkeletalMesh) (.weaponskin (Utilities|Array|Get(acopy) (Variables|Default|GetWeaponBoxMystery) (Variables|Default|GetIndex)))))

(fn ConstructionScript
  (Actor|Tick|SetActorTickInterval (Variables|Default|GetTick%20Interval)))

(fn GetInteractable
  (return "NewEnumerator1"))

(fn GetPossibleInteraction
  (return false))