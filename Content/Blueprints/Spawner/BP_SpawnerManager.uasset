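; BP_SpawnerManager runs server-side zombie waves, starting after a short delay when zombie activation is enabled.
; A looping timer spawns zombies at random GameMode spawn points with free barricade slots, up to a concurrent cap.
; Each zombie fills a slot, heads for the player or barricade depending on whether it is open, and gets wave-scaled health.
; When the active list empties, the next wave grows the zombie count and notifies the GameState.
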(event Custom|Spawner
  (bind _as_bp_game_mode_wave (Variables|Default|GetAs%20BP%20Game%20Mode%20Wave))
  (bind _spawnpointpossible (Variables|/Game/Blueprints/BP_Proto_GameMode_Wave.BP_Proto_GameMode_Wave_C|GetSpawnPointPossible _as_bp_game_mode_wave))
  (if (and (!= (Variables|Default|GetCounterAI) 0) (< (Utilities|Array|Length (Variables|Default|GetZombies)) (Variables|Default|GetZombiesSpawnMax)))
    (if (Utilities|Array|IsValidIndex _spawnpointpossible)
      (bind _output_get (Variables|Default|SetSpawnPoint (.OutItem (Utilities|Array|Random _spawnpointpossible))))
      (Utilities|IsValid _output_get
        (:Is%20Valid
          (if (Variables|/Game/Blueprints/Barricade/BP_Barricade.BP_Barricade_C|GetbIsOpen (Variables|/Game/Blueprints/Spawner/BP_SpawnerPoint.BP_SpawnerPoint_C|GetRefBarricade (Variables|Default|GetSpawnPoint)))
            _
            (else
              _))
          (bind (_useable _outitem) (Default|CheckZombieSlot (Variables|/Game/Blueprints/Spawner/BP_SpawnerPoint.BP_SpawnerPoint_C|GetRefBarricade (Variables|Default|GetSpawnPoint))))
          (if _useable
            (bind _returnvalue (Game|SpawnActorfromClass "/Game/Blueprints/Characters/Zombie/BP_Zombie.BP_Zombie_C" (Math|Transform|MakeTransform (Transformation|GetActorLocation (Variables|Default|GetSpawnPoint)) "0, 0, 0" "1.000000,1.000000,1.000000") "Undefined" "MultiplyWithRoot" 0 self 0 0))
            (Utilities|IsValid _returnvalue
              (:Is%20Valid
                (Variables|/Game/Blueprints/Characters/Zombie/BP_Zombie.BP_Zombie_C|SetAs%20BP%20Barricade _returnvalue (Variables|/Game/Blueprints/Spawner/BP_SpawnerPoint.BP_SpawnerPoint_C|GetRefBarricade (Variables|Default|GetSpawnPoint)))
                (Utilities|Array|Add (Variables|Default|GetZombies) _returnvalue)
                (Development|PrintString (Utilities|String|Append (Utilities|GetDisplayName (Variables|/Game/Blueprints/Spawner/BP_SpawnerPoint.BP_SpawnerPoint_C|GetRefBarricade (Variables|Default|GetSpawnPoint))) " Slot : " (Utilities|String|ToString(Integer) _outitem)))
                (Utilities|Array|SetArrayElem (Variables|/Game/Blueprints/Barricade/BP_Barricade.BP_Barricade_C|GetZombiesSlots (Variables|/Game/Blueprints/Spawner/BP_SpawnerPoint.BP_SpawnerPoint_C|GetRefBarricade (Variables|Default|GetSpawnPoint))) _outitem _returnvalue)
                (Math|Integer|DecrementInt (Variables|Default|GetCounterAI)
                  (:%20%20
                    (bind _refbarricade (Variables|/Game/Blueprints/Spawner/BP_SpawnerPoint.BP_SpawnerPoint_C|GetRefBarricade (Variables|Default|GetSpawnPoint))
                      (:then
                        (if (Variables|/Game/Blueprints/Barricade/BP_Barricade.BP_Barricade_C|GetbIsOpen _refbarricade)
                          (Default|Move _returnvalue "0, 0, 0" (Game|GetPlayerCharacter 0) "NewEnumerator2")
                          (else
                            (Default|MoveBarricade _returnvalue (Transformation|GetWorldLocation (Utilities|Array|Get(acopy) (Variables|/Game/Blueprints/Barricade/BP_Barricade.BP_Barricade_C|GetSlots (Variables|/Game/Blueprints/Spawner/BP_SpawnerPoint.BP_SpawnerPoint_C|GetRefBarricade (Variables|Default|GetSpawnPoint))) _outitem)) (Variables|/Game/Blueprints/Spawner/BP_SpawnerPoint.BP_SpawnerPoint_C|GetRefBarricade (Variables|Default|GetSpawnPoint)) "NewEnumerator1")))
                        (Variables|/Game/Blueprints/Composents/AC_Stats.AC_Stats_C|SetHealth (Variables|/Game/Blueprints/Characters/Zombie/BP_Zombie.BP_Zombie_C|GetBP_Stats _returnvalue) (* (Variables|Default|GetWave) 1e+02)))
                      (:else))))))))))))

(event Custom|Remove%20Zombies
  (params (Zombie :type BP%20Zombie%20Object%20Reference%20%28by%20ref%29))
  (bind _zombies (Variables|Default|GetZombies))
  (Utilities|Array|RemoveItem _zombies Zombie)
  (if (== (Utilities|Array|Length _zombies) 0)
    (CallFunction|NewWave)))

(event Custom|NewWave
  (bind _as_bp_proto_game_state_wave (Variables|Default|GetAs%20BP%20Proto%20Game%20State%20Wave))
  (Development|PrintString "New Wave")
  (Math|Integer|IncrementInt (Variables|Default|GetWave)
    (:%20%20
      (bind _output_get (Variables|Default|SetNbAiWave (* (Variables|Default|GetNbAiWave) (Variables|Default|GetWave))))
      (Variables|Default|SetCounterAI _output_get)
      (Variables|/Game/Blueprints/BP_Proto_GameState_Wave.BP_Proto_GameState_Wave_C|SetWave _as_bp_proto_game_state_wave (Variables|Default|GetWave))
      (Default|CallOnChangeWaves _as_bp_proto_game_state_wave))))

(event EventBeginPlay
  (Utilities|FlowControl|Delay 5.0)
  (if (Variables|Default|GetbActivatedZombie)
    (Networking|SwitchHasAuthority
      (:Authority
        (bind _asbp_proto_game_mode_wave (Utilities|Casting|CastToBP_Proto_GameMode_Wave (Game|GetGameMode)))
        (Variables|Default|SetAs%20BP%20Game%20Mode%20Wave _asbp_proto_game_mode_wave)
        (bind _asbp_proto_game_state_wave (Utilities|Casting|CastToBP_Proto_GameState_Wave (Game|GetGameState)))
        (Variables|Default|SetAs%20BP%20Proto%20Game%20State%20Wave _asbp_proto_game_state_wave)
        (Variables|Default|SetCounterAI (Variables|Default|GetNbAiWave))
        (Variables|Default|SetWave 1)
        (bind _returnvalue (Utilities|Time|SetTimerbyEvent (delegate Custom|Spawner) 1.0 true))
        (Variables|Default|Sethandle _returnvalue)))))

(fn ConstructionScript)