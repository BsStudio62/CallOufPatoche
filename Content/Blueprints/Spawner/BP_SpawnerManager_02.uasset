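; Wave-based zombie spawner that, when activated, starts on the server shortly after BeginPlay.
; A looping timer spawns BP_Zombie at the manager's location while the wave budget remains and the live count is under a cap, passing itself as Spawner.
; RemoveZombies starts a new wave whenever the live list empties, multiplying the previous wave size by the new wave number.
; Game state wave update nodes exist but are disconnected.
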(event Custom|Spawner
  (if (and (!= (Variables|Default|GetCounterAI) 0) (< (Utilities|Array|Length (Variables|Default|GetZombies)) (Variables|Default|GetZombiesSpawnMax)))
    (bind _returnvalue (Game|SpawnActorfromClass "/Game/Blueprints/BP_Zombie.BP_Zombie_C" (Math|Transform|MakeTransform (Transformation|GetActorLocation) "0, 0, 0" "1.000000,1.000000,1.000000") "Undefined" "MultiplyWithRoot" 0 self 0))
    (Utilities|IsValid _returnvalue
      (:Is%20Valid
        (Utilities|Array|Add (Variables|Default|GetZombies) _returnvalue)
        (Math|Integer|DecrementInt (Variables|Default|GetCounterAI))))))

(event Custom|Remove%20Zombies
  (params (Zombie :type BP%20Zombie%20Object%20Reference%20%28by%20ref%29))
  (bind _zombies (Variables|Default|GetZombies))
  (Utilities|Array|RemoveItem _zombies Zombie)
  (if (== (Utilities|Array|Length _zombies) 0)
    (CallFunction|NewWave)))

(event Custom|NewWave
  (Development|PrintString "New Wave")
  (Math|Integer|IncrementInt (Variables|Default|GetWave)
    (:%20%20
      (bind _output_get (Variables|Default|SetNbAiWave (* (Variables|Default|GetNbAiWave) (Variables|Default|GetWave))))
      (Variables|Default|SetCounterAI _output_get))))

(event EventBeginPlay
  (Utilities|FlowControl|Delay 1.0)
  (if (Variables|Default|GetbActivatedZombie)
    (Networking|SwitchHasAuthority
      (:Authority
        (Variables|Default|SetCounterAI (Variables|Default|GetNbAiWave))
        (Variables|Default|SetWave 1)
        (bind _returnvalue (Utilities|Time|SetTimerbyEvent (delegate Custom|Spawner) 1.0 true))
        (Variables|Default|Sethandle _returnvalue)))))

(fn ConstructionScript)