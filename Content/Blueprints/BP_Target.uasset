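; BP_Target is a target actor that reacts to its Damage event by losing its head temporarily.
; The event hides the skeletal mesh's "head" bone, waits five seconds through a Delay, then unhides it.
; Separately, it listens to the AC_Attribute component's OnHealthChanged event and prints health and delta as debug text, without driving the head effect.
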(event OnHealthChanged(AC_Attribute)
  (params (OwningHealthComp :type S%20Attribute%20Component%20Object%20Reference) (Health :type Float%20%28single-precision%29) (HealthDelta :type Float%20%28single-precision%29) (DamageType :type Damage%20Type%20Object%20Reference) (InstigatedBy :type Controller%20Object%20Reference) (DamageCauser :type Actor%20Object%20Reference))
  (Development|PrintString (Utilities|String|Append "Health : " (Utilities|String|ToString(Float) Health) " Health Delta : " (Utilities|String|ToString(Float) HealthDelta))))

(event EventDamage
  (params (Damage :type Float%20%28double-precision%29))
  (Components|SkinnedMesh|HideBonebyName (Variables|Default|GetSkeletalMesh) "head" "PBO_None")
  (Utilities|FlowControl|Delay 5.0)
  (Components|SkinnedMesh|UnHideBonebyName (Variables|Default|GetSkeletalMesh) "head"))

(fn ConstructionScript)