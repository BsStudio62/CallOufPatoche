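; Behavior tree service for zombie AI that tracks the distance to the player.
; On activation it sets the Target blackboard key to the first player character and seeds Range with a large default.
; Each tick it writes the controlled pawn's distance to a valid Target into Range.
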(event EventReceiveTickAI
  (params (OwnerController :type AI%20Controller%20Object%20Reference) (ControlledPawn :type Pawn%20Object%20Reference) (DeltaSeconds :type Float%20%28single-precision%29))
  (bind _target (Variables|Default|GetTarget))
  (bind _returnvalue (AI|BehaviorTree|GetBlackboardValueasActor _target))
  (Utilities|IsValid _returnvalue
    (:Is%20Valid
      (Class|BTFunctionLibrary|SetBlackboardValueasFloat (Variables|Default|GetRange) (Transformation|GetDistanceTo ControlledPawn _returnvalue)))))

(event EventReceiveActivation
  (params (OwnerActor :type Actor%20Object%20Reference))
  (Class|BTFunctionLibrary|SetBlackboardValueasFloat (Variables|Default|GetRange) 1e+03)
  (Class|BTFunctionLibrary|SetBlackboardValueasObject (Variables|Default|GetTarget) (Game|GetPlayerCharacter 0)))