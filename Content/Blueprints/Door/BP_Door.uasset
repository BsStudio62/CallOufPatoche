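; BP_Door is an interactable door that deducts 100 points from the interacting player and is then removed.
; Interaction charges the player state and refreshes the HUD through the player controller, with no affordability check in this graph.
; It activates its linked SpawnPoint if valid and destroys itself.
; It also calls BP_GameModeWave's CallOnActorKilled, passing the interacting player's state as the killer.
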(event EventInteraction
  (params (PC :type Player%20Controller%20Object%20Reference))
  (bind _playerstate (Variables|/Script/Engine.Controller|GetPlayerState PC))
  (bind _assplayer_state (Utilities|Casting|CastToSPlayerState _playerstate))
  (Class|SPlayerState|RemovePoints _assplayer_state 100)
  (Default|CallOnUpdateHud (.AsSPlayer%20Controller (Utilities|Casting|CastToSPlayerController PC)))
  (Utilities|FlowControl|Sequence
    (:then_0
      (bind _spawnpoint (Variables|Default|GetSpawnPoint)
        (:then
          (Class|SSpawnPoint|SetActivated _spawnpoint true))
        (:else
          _))
      (Actor|DestroyActor))
    (:then_1
      (bind _asbp_game_mode_wave (Utilities|Casting|CastToBP_GameModeWave (Game|GetGameMode)))
      (Default|CallOnActorKilled _asbp_game_mode_wave 0 0 0 _assplayer_state))))

(fn ConstructionScript)