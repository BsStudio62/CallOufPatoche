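; Skybox Blueprint that drives a panning-cloud sky sphere material and switches between Sun and Moon lights.
; The construction script creates the dynamic material and maps Sun pitch to SunHeight, which selects curve-based colors unless manual colors apply.
; A negative height blends in stars and shows the Moon instead of the Sun.
; UpdateSunDirection refreshes only sun-driven parameters, always using curves, and is not called within this graph.
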(fn ConstructionScript
  (bind _returnvalue (Rendering|Material|CreateDynamicMaterialInstance (Variables|BP_Skydome|GetSkySphereMesh) 0 "/Engine/EngineSky/M_Sky_Panning_Clouds2.M_Sky_Panning_Clouds2" "None" :!class /Script/Engine.PrimitiveComponent))
  (Variables|Default|SetSky%20material _returnvalue)
  (if (Variables|Default|GetRefresh%20material) ; Updating bool in details panel causes construction script to run again
    _
    (else
      _))
  (Variables|Default|SetRefresh%20material false)
  (CallFunction|RefreshMaterial)
  (CallFunction|MoonandSun)
  (CallFunction|SettingMoon))

(fn UpdateSunDirection
  (bind _sky_material (Variables|Default|GetSky%20material))
  (bind _sky_material_2 (Variables|Default|GetSky%20material))
  (Rendering|Material|SetVectorParameterValue _sky_material "Light direction" (Math|Conversions|ToLinearColor(Vector) (Math|Rotator|GetRotationXVector (Transformation|GetWorldRotation (Variables|Default|GetSun)))) :!class /Script/Engine.MaterialInstanceDynamic)
  (Rendering|Material|SetVectorParameterValue _sky_material "Sun color" (Math|Conversions|ToLinearColor(Color) (Variables|/Script/Engine.LightComponentBase|GetLightColor (Variables|Default|GetSun))) :!class /Script/Engine.MaterialInstanceDynamic)
  (Variables|Overridesettings|SetSun%20height (Math|Float|MapRangeUnclamped (.Pitch (Math|Rotator|BreakRotator (Transformation|GetWorldRotation (Variables|Default|GetSun)))) 0.0 -9e+01 0.0 1.0))
  (Rendering|Material|SetVectorParameterValue _sky_material_2 "Horizon color" (Class|CurveLinearColor|GetClampedLinearColorValue (Variables|Default|GetHorizon%20color%20curve) (Variables|Overridesettings|GetSun%20height)) :!class /Script/Engine.MaterialInstanceDynamic)
  (Rendering|Material|SetVectorParameterValue _sky_material_2 "Zenith color" (Class|CurveLinearColor|GetClampedLinearColorValue (Variables|Default|GetZenith%20color%20curve) (Variables|Overridesettings|GetSun%20height)) :!class /Script/Engine.MaterialInstanceDynamic)
  (Rendering|Material|SetVectorParameterValue _sky_material_2 "Cloud color" (Class|CurveLinearColor|GetClampedLinearColorValue (Variables|Default|GetCloud%20color%20curve) (Variables|Overridesettings|GetSun%20height)) :!class /Script/Engine.MaterialInstanceDynamic)
  (Rendering|Material|SetScalarParameterValue _sky_material_2 "Horizon falloff" (Math|Float|Lerp 3.0 8.0 (Math|Float|Absolute(Float) (Variables|Overridesettings|GetSun%20height))) :!class /Script/Engine.MaterialInstanceDynamic)
  (Rendering|Material|SetScalarParameterValue _sky_material_2 "Sun height" (Math|Float|SelectFloat (Math|Float|Absolute(Float) (Variables|Overridesettings|GetSun%20height)) 0.0 (< (Variables|Overridesettings|GetSun%20height) 0.0)) :!class /Script/Engine.MaterialInstanceDynamic))

(fn RefreshMaterial
  (bind _sky_material (Variables|Default|GetSky%20material))
  (bind _sky_material_2 (Variables|Default|GetSky%20material))
  (bind _sky_material_3 (Variables|Default|GetSky%20material))
  (bind _sky_material_4 (Variables|Default|GetSky%20material))
  (Rendering|Material|SetVectorParameterValue _sky_material_2 "Light direction" (Math|Conversions|ToLinearColor(Vector) (Math|Rotator|GetRotationXVector (Transformation|GetWorldRotation (Variables|Default|GetSun)))) :!class /Script/Engine.MaterialInstanceDynamic)
  (Rendering|Material|SetVectorParameterValue _sky_material_2 "Sun color" (Math|Conversions|ToLinearColor(Color) (Variables|/Script/Engine.LightComponentBase|GetLightColor (Variables|Default|GetSun))) :!class /Script/Engine.MaterialInstanceDynamic)
  (Variables|Overridesettings|SetSun%20height (Math|Float|MapRangeUnclamped (.Pitch (Math|Rotator|BreakRotator (Transformation|GetWorldRotation (Variables|Default|GetSun)))) 0.0 -9e+01 0.0 1.0))
  (if (Variables|Default|GetColors%20determined%20by%20sun%20position)
    (Rendering|Material|SetVectorParameterValue _sky_material_3 "Horizon color" (Class|CurveLinearColor|GetClampedLinearColorValue (Variables|Default|GetHorizon%20color%20curve) (Variables|Overridesettings|GetSun%20height)) :!class /Script/Engine.MaterialInstanceDynamic)
    (Rendering|Material|SetVectorParameterValue _sky_material_3 "Zenith color" (Class|CurveLinearColor|GetClampedLinearColorValue (Variables|Default|GetZenith%20color%20curve) (Variables|Overridesettings|GetSun%20height)) :!class /Script/Engine.MaterialInstanceDynamic)
    (Rendering|Material|SetVectorParameterValue _sky_material_3 "Cloud color" (Class|CurveLinearColor|GetClampedLinearColorValue (Variables|Default|GetCloud%20color%20curve) (Variables|Overridesettings|GetSun%20height)) :!class /Script/Engine.MaterialInstanceDynamic)
    (Rendering|Material|SetScalarParameterValue _sky_material_3 "Horizon falloff" (Math|Float|Lerp 3.0 7.0 (Math|Float|Absolute(Float) (Variables|Overridesettings|GetSun%20height))) :!class /Script/Engine.MaterialInstanceDynamic)
    (else
      (Rendering|Material|SetVectorParameterValue _sky_material "Horizon color" (Variables|Overridesettings|GetHorizon%20color) :!class /Script/Engine.MaterialInstanceDynamic)
      (Rendering|Material|SetVectorParameterValue _sky_material "Zenith color" (Variables|Overridesettings|GetZenith%20Color) :!class /Script/Engine.MaterialInstanceDynamic)
      (Rendering|Material|SetVectorParameterValue _sky_material "Overall color" (Variables|Overridesettings|GetOverall%20Color) :!class /Script/Engine.MaterialInstanceDynamic)
      (Rendering|Material|SetVectorParameterValue _sky_material "Cloud color" (Variables|Overridesettings|GetCloud%20color) :!class /Script/Engine.MaterialInstanceDynamic)
      (Rendering|Material|SetScalarParameterValue _sky_material "Horizon falloff" (Variables|Overridesettings|GetHorizon%20Falloff) :!class /Script/Engine.MaterialInstanceDynamic)))
  (Rendering|Material|SetScalarParameterValue _sky_material_4 "Cloud speed" (Variables|Default|GetCloud%20speed) :!class /Script/Engine.MaterialInstanceDynamic)
  (Rendering|Material|SetScalarParameterValue _sky_material_4 "Sun brightness" (Variables|Default|GetSun%20brightness) :!class /Script/Engine.MaterialInstanceDynamic)
  (Rendering|Material|SetScalarParameterValue _sky_material_4 "Sun height" (Math|Float|SelectFloat (Math|Float|Absolute(Float) (Variables|Overridesettings|GetSun%20height)) 0.0 (< (Variables|Overridesettings|GetSun%20height) 0.0)) :!class /Script/Engine.MaterialInstanceDynamic)
  (Rendering|Material|SetScalarParameterValue _sky_material_4 "Cloud opacity" (Variables|Default|GetCloud%20opacity) :!class /Script/Engine.MaterialInstanceDynamic)
  (Rendering|Material|SetScalarParameterValue _sky_material_4 "Stars brightness" (Variables|Default|GetStars%20brightness) :!class /Script/Engine.MaterialInstanceDynamic))

(fn MoonandSun
  (if (< (Variables|Overridesettings|GetSun%20height) 0.0)
    (Rendering|SetVisibility (Variables|Default|GetSun) false false)
    (Rendering|SetVisibility (Variables|Default|GetMoon) true false)
    (else
      (Rendering|SetVisibility (Variables|Default|GetSun) true false)
      (Rendering|SetVisibility (Variables|Default|GetMoon) false false))))

(fn SettingMoon
  (Rendering|Components|Light|SetIntensity (Variables|Default|GetMoon) (Variables|Moon|GetIntensityMoon)))