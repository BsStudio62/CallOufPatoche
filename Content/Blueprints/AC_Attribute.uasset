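; AC_Attribute is a health component Blueprint that awards score for damage and handles the owner's death and revival.
; On the server it binds to health changes, adds points to the instigator's SPlayerState on each change, and tells that player's BP_PlayerController to update its HUD.
; Dead destroys the owner, while Revive resets health and unhides it.
; A hide-then-delayed-revive sequence is left disconnected.
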(event Custom|CustomEvent
  (params (OwningHealthComp :type S%20Attribute%20Component%20Object%20Reference) (Health :type Float%20%28single-precision%29) (HealthDelta :type Float%20%28single-precision%29) (DamageType :type Damage%20Type%20Object%20Reference) (InstigatedBy :type Controller%20Object%20Reference) (DamageCauser :type Actor%20Object%20Reference))
  (bind _playerstate (Variables|/Script/Engine.Controller|GetPlayerState InstigatedBy))
  (bind (_assplayer_state _bsuccess) (Utilities|Casting|CastToSPlayerState _playerstate))
  (if _bsuccess
    (Class|SPlayerState|AddPoints _assplayer_state 10)
    (if (Networking|IsServer)
      (bind _asbp_player_controller (Utilities|Casting|CastToBP_PlayerController InstigatedBy))
      (Class|SPlayerController|ClientUpdateHud _asbp_player_controller))))

(event EventBeginPlay
  (Networking|SwitchHasAuthority
    (:Authority
      (EventDispatchers|BindEventtoOnHealthChanged (delegate Custom|CustomEvent)))))

(event EventRevive
  (Class|SAttributeComponent|ResetHealth)
  (Rendering|SetActorHiddenInGame (Components|GetOwner) false))

(event EventDead
  (Actor|DestroyActor (Components|GetOwner)))