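; Zombie-window style barricade of five BP_Plank child actors that can be removed and rebuilt one at a time.
; An index steps through the planks, playing their timelines forward to remove and in reverse to rebuild, driven by Tick's Build flag or player Interact.
; A trigger box registers itself as the player's interaction and flags zombies as inside the building on entry, freeing their slot on exit.
; Helper functions pick random free zombie slots and clear them.
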(event OnComponentBeginOverlap(Box)
  (params (OverlappedComponent :type Primitive%20Component%20Object%20Reference) (OtherActor :type Actor%20Object%20Reference) (OtherComp :type Primitive%20Component%20Object%20Reference) (OtherBodyIndex :type Integer) (bFromSweep :type Boolean) (SweepResult :type Hit%20Result%20Structure%20%28by%20ref%29))
  (bind _asbp_proto_player (Utilities|Casting|CastToBP_Proto_Player OtherActor)
    (:then
      (Variables|/Game/Blueprints/Characters/Proto/BP_Proto_Player.BP_Proto_Player_C|SetInteraction _asbp_proto_player self))
    (:CastFailed
      (bind _asbp_zombie (Utilities|Casting|CastToBP_Zombie OtherActor))
      (Variables|/Game/Blueprints/Characters/Zombie/BP_Zombie.BP_Zombie_C|SetInBuilding _asbp_zombie true))))

(event OnComponentEndOverlap(Box)
  (params (OverlappedComponent :type Primitive%20Component%20Object%20Reference) (OtherActor :type Actor%20Object%20Reference) (OtherComp :type Primitive%20Component%20Object%20Reference) (OtherBodyIndex :type Integer))
  (bind _asbp_proto_player (Utilities|Casting|CastToBP_Proto_Player OtherActor)
    (:then
      (Variables|/Game/Blueprints/Characters/Proto/BP_Proto_Player.BP_Proto_Player_C|SetInteraction _asbp_proto_player 0))
    (:CastFailed
      (bind _asbp_zombie (Utilities|Casting|CastToBP_Zombie OtherActor))
      (CallFunction|RemoveZombieSlot _asbp_zombie))))

(event Custom|Add%20Barricade
  (if (!= (Variables|Default|GetIndex) -1)
    (if (== (Variables|Default|GetIndex) 5)
      (Variables|Default|SetIndex 4))
    (bind _asbp_plank (Utilities|Casting|CastToBP_Plank (Variables|/Script/Engine.ChildActorComponent|GetChildActor (Utilities|Array|Get(acopy) (Utilities|Array|MakeArray (Variables|Default|GetChildActor) (Variables|Default|GetChildActor1) (Variables|Default|GetChildActor2) (Variables|Default|GetChildActor3) (Variables|Default|GetChildActor4)) (Variables|Default|GetIndex)))))
    (Components|Timeline|SetPlayRate (Variables|/Game/Blueprints/Barricade/BP_Plank.BP_Plank_C|GetTimeline _asbp_plank) 1.0)
    (Utilities|String|Reverse (Variables|/Game/Blueprints/Barricade/BP_Plank.BP_Plank_C|GetTimeline _asbp_plank))
    (bind _result (Math|Integer|DecrementInt (Variables|Default|GetIndex))
      (:%20%20
        (Variables|Default|SetbIsOpen false)
        (if (== _result -1)
          (Variables|Default|SetIndex 0)
          (Actor|Tick|SetActorTickEnabled false))))))

(event Custom|Remove%20Barricade
  (if (Variables|Default|GetbIsOpen)
    (Actor|Tick|SetActorTickEnabled false :!label _label)
    (else
      (bind _asbp_plank (Utilities|Casting|CastToBP_Plank (Variables|/Script/Engine.ChildActorComponent|GetChildActor (Utilities|Array|Get(acopy) (Utilities|Array|MakeArray (Variables|Default|GetChildActor) (Variables|Default|GetChildActor1) (Variables|Default|GetChildActor2) (Variables|Default|GetChildActor3) (Variables|Default|GetChildActor4)) (Variables|Default|GetIndex)))))
      (Components|Timeline|SetPlayRate (Variables|/Game/Blueprints/Barricade/BP_Plank.BP_Plank_C|GetTimeline _asbp_plank) 1.0)
      (Audio|Components|Audio|Play (Variables|/Game/Blueprints/Barricade/BP_Plank.BP_Plank_C|GetTimeline _asbp_plank))
      (bind _result (Math|Integer|IncrementInt (Variables|Default|GetIndex))
        (:%20%20
          (bind _output_get (Variables|Default|SetbIsOpen (> _result 4)))
          (if _output_get
            (goto _label)
            (else
              _))))))
  (for _array_element (Utilities|Array|MakeArray (Variables|Default|GetChildActor) (Variables|Default|GetChildActor1) (Variables|Default|GetChildActor2) (Variables|Default|GetChildActor3) (Variables|Default|GetChildActor4))
    (bind _asbp_plank_2 (Utilities|Casting|CastToBP_Plank (Variables|/Script/Engine.ChildActorComponent|GetChildActor _array_element)))
    (Collision|SetCollisionEnabled (Variables|/Game/Blueprints/Barricade/BP_Plank.BP_Plank_C|GetCube _asbp_plank_2) "NoCollision")))

(event EventInteract
  (params (Player :type BP%20Proto%20Player%20Object%20Reference))
  (Development|PrintString "Barricade")
  (CallFunction|AddBarricade))

(event EventTick
  (params (DeltaSeconds :type Float%20%28single-precision%29))
  (if (Variables|Default|GetBuild)
    (CallFunction|AddBarricade)
    (else
      (CallFunction|RemoveBarricade))))

(fn ConstructionScript
  (Variables|Default|SetSlots (Utilities|Array|MakeArray (Variables|Default|GetSlot01) (Variables|Default|GetSlot02) (Variables|Default|GetSlot03))))

(fn CheckZombieSlot
  (bind _slotsindex (LocalVariables|GetSlotsIndex))
  (for (_array_element _array_index) (Variables|Default|GetZombiesSlots)
    (Utilities|IsValid _array_element
      (:Is%20Not%20Valid
        (Utilities|Array|Add (LocalVariables|GetSlotsIndex) _array_index))))
  (if (Utilities|Array|IsEmpty _slotsindex)
    (return false 0)
    (else
      (return true (.OutItem (Utilities|Array|Random _slotsindex))))))

(fn ClearZombies
  (bind _zombiesslots (Variables|Default|GetZombiesSlots))
  (bind _index (Utilities|FlowControl|ForLoopwithBreak 0 (Utilities|Array|Length _zombiesslots))
    (:LoopBody
      (Utilities|Array|SetArrayElem _zombiesslots _index 0))))

(fn RemoveZombieSlot
  (params (Zombie :type BP%20Zombie%20Object%20Reference%20%28by%20ref%29))
  (bind _zombiesslots (Variables|Default|GetZombiesSlots))
  (bind _returnvalue (Utilities|Array|FindItem _zombiesslots Zombie))
  (Development|PrintString (Utilities|String|Append (Utilities|GetDisplayName Zombie) " / " (Utilities|String|ToString(Integer) _returnvalue)))
  (Utilities|Array|SetArrayElem _zombiesslots _returnvalue 0))

(fn GetInteractable
  (return (Variables|Default|GetInteraction)))

(fn GetPossibleInteraction
  (return (!= (Variables|Default|GetIndex) 0)))