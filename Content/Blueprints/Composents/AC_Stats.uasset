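; Stats component that handles health, damage and death for both AI zombies and players, binding its damage handler on the server.
; Damage lowers Health and broadcasts the change; AI hits set the attacker's score, with kills scored by hit surface type.
; Dead AI owners are destroyed, while dead players are only flagged.
; Surviving players regenerate through a delayed looping timer that stops at full health.
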(event Custom|Retrieve%20Health
  (Development|PrintString "RegenHealth")
  (bind _output_get (Variables|Default|SetHealth (Math|Float|Clamp(Float) (+ (Variables|Default|GetHealth) (Variables|Default|GetRegenHealth)) 0.0 1e+02)))
  (Default|CallOnHealthChanged)
  (if (== _output_get 1e+02)
    (Utilities|Time|ClearandInvalidateTimerbyHandle (Variables|Default|GetHandle))))

(event Custom|OnHealthDamaged_Event
  (params (Damage :type Float%20%28double-precision%29) (ZoneDamage :type EPhysicalSurface%20Enum :default "SurfaceType_Default") (PlayerState :type BP%20Proto%20Player%20State%20Object%20Reference))
  (bind _output_get (Variables|Default|SetHealth (- (Variables|Default|GetHealth) Damage)))
  (Default|CallOnHealthChanged)
  (if (<= _output_get 0.0)
    (if (Variables|Default|GetAI)
      (Default|SetScore PlayerState (Math|Float|SelectFloat 5e+01 1e+01 (Utilities|Enum|Equal(Enum) ZoneDamage "SurfaceType1")))
      (Development|PrintString "Zombie")
      (Actor|DestroyActor (Components|GetOwner))
      (else
        (Variables|Default|SetbIsDead true)
        (Development|PrintString "Dead Player")))
    (elif (Variables|Default|GetAI)
      (Default|SetScore PlayerState 1e+01)
      (else
        (CallFunction|HealthTimer)))))

(event Custom|HealthTimer
  (Development|PrintString "LauncheTimer")
  (bind _returnvalue (Utilities|Time|SetTimerbyEvent (delegate Custom|Retrieve%20Health) 0.5 true 5.0))
  (Variables|Default|SetHandle _returnvalue))

(event EventBeginPlay
  (Networking|SwitchHasAuthority
    (:Authority
      (EventDispatchers|BindEventtoOnHealthDamaged (delegate Custom|OnHealthDamaged_Event)))))