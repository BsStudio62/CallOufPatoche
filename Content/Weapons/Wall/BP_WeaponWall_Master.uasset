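; Master Blueprint for a wall weapon that swaps the player's current weapon when they interact and have enough points.
; Interaction checks player-state points against Cost but does not deduct them, then destroys the held weapon.
; It spawns WeaponClass, snaps it to the first-person mesh at a socket from class defaults, and makes it current.
; It clears owner-only visibility on both weapon meshes, then initializes the new weapon's input after a short delay.
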(event EventInteraction
  (params (PC :type Player%20Controller%20Object%20Reference))
  (bind _weaponclass (Variables|Default|GetWeaponClass))
  (bind _assplayer_state (Utilities|Casting|CastToSPlayerState (Variables|/Script/Engine.Controller|GetPlayerState PC)))
  (if (>= (Class|SPlayerState|GetPoints _assplayer_state) (Variables|Default|GetCost))
    (bind _asbp_player (Utilities|Casting|CastToBP_Player (Pawn|GetControlledPawn PC)))
    (Actor|DestroyActor (Variables|/Script/CallOufPatoche.SCharacter|GetCurrentWeapon _asbp_player))
    (bind _returnvalue (Game|SpawnActorfromClass _weaponclass (Math|Transform|MakeTransform "0, 0, 0" "0, 0, 0" "1.000000,1.000000,1.000000") "Undefined" "MultiplyWithRoot" 0 0))
    (Transformation|AttachComponentToComponent _returnvalue (Class|SCharacter|GetMesh1P _asbp_player) (Utilities|GetClassDefaults _weaponclass) "SnapToTarget" "SnapToTarget" "SnapToTarget" true)
    (bind _output_get (Variables|/Script/CallOufPatoche.SCharacter|SetCurrentWeapon _asbp_player _returnvalue))
    (Rendering|SetOnlyOwnerSee (Variables|Default|GetWeapon) false :!class /Script/Engine.PrimitiveComponent)
    (Utilities|FlowControl|Delay 1.0)
    (Class|SWeapon|SetupInputSystem _output_get)))

(fn ConstructionScript)