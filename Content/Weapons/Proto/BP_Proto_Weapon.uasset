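; Prototype hitscan firearm for the first-person player, handling firing, reloading and ammo.
; Fire and reload route to the server; a timer paced by fire rate, looping per fire mode, drives each shot.
; Shots play montages and camera shake, trace from the eye viewpoint, draw debug shapes, push physics objects and damage AC_Stats by surface type.
; Reload montage completion moves reserve rounds into the magazine; ammo changes refresh the HUD weapon widget.
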(event Custom|Fire
  (Networking|SwitchHasAuthority
    (:Authority
      (Development|PrintString "Fire" false false)
      (if (CallFunction|CheckMunition)
        (if (not (Class|KismetSystemLibrary|TimerExistsHandle (Variables|Default|GethandleFire)))
          (bind _returnvalue (Utilities|Time|SetTimerbyEvent (delegate Custom|CustomEvent) (Variables|Default|GetTimeBetweenShot) (Variables|Default|GetFireMod) (Math|Float|Max(Float) (- (+ (Variables|Default|GetLastFireTime) (Variables|Default|GetTimeBetweenShot)) (Utilities|Time|GetTimeSeconds)) 0.0)))
          (Variables|Default|SethandleFire _returnvalue)
          (if (not (Variables|Default|GetCurrentFire))
            (Variables|Default|SetCurrentFire false)))))
    (:Remote
      (CallFunction|ServerFire))))

(event Custom|CustomEvent
  (bind _returnvalue (Components|GetOwner))
  (bind _player (Variables|Default|GetPlayer))
  (bind _montage_fire_arms (Variables|Animation|Arms|GetMontage%20Fire%20Arms))
  (bind (_outlocation _outrotation) (Actor|GetActorEyesViewPoint _returnvalue))
  (bind _firstpersonmesh (Variables|/Game/Blueprints/Characters/Proto/BP_Proto_Player.BP_Proto_Player_C|GetFirstPersonMesh _player))
  (bind _asplayer_controller (Utilities|Casting|CastToPlayerController (Game|GetInstigatorController (Components|GetOwner))))
  (Game|Feedback|ClientStartCameraShake _asplayer_controller "/Game/Blueprints/CameraShake/BP_CameraShake.BP_CameraShake_C" 1.0 "CameraLocal" "0, 0, 0")
  (if (Variables|/Game/Blueprints/Characters/Proto/BP_Proto_Player.BP_Proto_Player_C|GetbIsADS _player)
    _
    (elif (Variables|Default|GetbMontageFire)
      (Animation|Montage|PlayMontage _firstpersonmesh _montage_fire_arms
        (:then
          (CallFunction|ClientMontage _montage_fire_arms _firstpersonmesh)))))
  ;[1 1 1] Animation Weapon
  (Animation|Montage|PlayMontage (Variables|Default|GetSkeletalMesh) (Variables|Animation|Weapon|GetMontage%20Fire%20Weapon)
    (:then
      (bind (_outhit _returnvalue_2) (Collision|LineTraceByChannel _outlocation (+ _outlocation (* (Math|Rotator|GetRotationXVector _outrotation) (Variables|Default|GetDistance))) "TraceTypeQuery3" false (Utilities|Array|MakeArray (Components|GetOwner) self) "None"))
      (Rendering|Debug|DrawDebugLine :LineStart (Transformation|GetSocketLocation (Variables|Default|GetSkeletalMesh) "Muzzle") :LineEnd (Math|Vector|SelectVector (.Location (Collision|BreakHitResult _outhit)) (.TraceEnd (Collision|BreakHitResult _outhit)) _returnvalue_2) :Duration 1.0)
      (Utilities|IsValid (.HitComponent (Collision|BreakHitResult _outhit))
        (:Is%20Valid
          (if (Physics|IsSimulatingPhysics (.HitComponent (Collision|BreakHitResult _outhit)) "None")
            (Physics|AddImpulseatLocation (.HitComponent (Collision|BreakHitResult _outhit)) (* (.ImpactPoint (Collision|BreakHitResult _outhit)) 1e+02) (.Location (Collision|BreakHitResult _outhit)) "None")))
        (:Is%20Not%20Valid
          _))
      (Utilities|IsValid (.PhysMat (Collision|BreakHitResult _outhit))
        (:Is%20Valid
          (switch Utilities|FlowControl|Switch|SwitchonEPhysicalSurface (Variables|/Script/PhysicsCore.PhysicalMaterial|GetSurfaceType (.PhysMat (Collision|BreakHitResult _outhit)))
            (:SurfaceType_Default
              (Rendering|Debug|DrawDebugSphere (.Location (Collision|BreakHitResult _outhit)) 1e+01 12 "(R=0.000000,G=1.000000,B=0.096722,A=1.000000)" 0.0))
            (:SurfaceType1
              (Rendering|Debug|DrawDebugSphere (.Location (Collision|BreakHitResult _outhit)) 1e+01 12 "(R=1.000000,G=0.000000,B=0.192791,A=1.000000)" 0.0)))
          ;[1 1 1] Dernier Tir effectuer
          (Variables|Default|SetLastFireTime (Utilities|Time|GetTimeSeconds))
          (Math|Integer|DecrementInt (Variables|Default|GetCurrentMunition)
            (:%20%20
              (Default|CallOnFireUpdate (Variables|/Game/Blueprints/Widget/WBP_Hud.WBP_Hud_C|GetWBP_Weapon (Variables|/Game/Blueprints/BP_FirstPersonPlayerController.BP_FirstPersonPlayerController_C|GetRefHud (Variables|Default|GetAs%20BP%20First%20Person%20Player%20Controller))))
              (Utilities|IsValid (.HitActor (Collision|BreakHitResult _outhit))
                (:Is%20Valid
                  (Utilities|IsValid (Actor|GetComponentbyClass (.HitActor (Collision|BreakHitResult _outhit)) "/Game/Blueprints/Composents/AC_Stats.AC_Stats_C")
                    (:Is%20Valid
                      (bind _asbp_proto_player_state (Utilities|Casting|CastToBP_Proto_PlayerState (Variables|/Script/Engine.Controller|GetPlayerState (Game|GetInstigatorController))))
                      (Default|CallOnHealthDamaged (Actor|GetComponentbyClass (.HitActor (Collision|BreakHitResult _outhit)) "/Game/Blueprints/Composents/AC_Stats.AC_Stats_C") (Utilities|Select :Index (Variables|/Script/PhysicsCore.PhysicalMaterial|GetSurfaceType (.PhysMat (Collision|BreakHitResult _outhit))) :SurfaceType_Default 1e+01 :SurfaceType1 1e+02 :SurfaceType2 0.0) (Variables|/Script/PhysicsCore.PhysicalMaterial|GetSurfaceType (.PhysMat (Collision|BreakHitResult _outhit))) _asbp_proto_player_state))))))))))
    (:OnCompleted
      (Variables|Default|SetCurrentFire false))))

(event Custom|Stop%20Fire
  (bind _handlefire (Variables|Default|GethandleFire))
  (if (and (Class|KismetSystemLibrary|TimerExistsHandle _handlefire) (Variables|Default|GetFireMod))
    (Utilities|Time|ClearandInvalidateTimerbyHandle _handlefire)))

(event Custom|Server_Fire
  (CallFunction|Fire))

(event Custom|Start%20Reload
  (Networking|SwitchHasAuthority
    (:Authority
      (Development|PrintString "Reload")
      (if (not (Math|Boolean|ANDBoolean (Variables|Default|GetbReloading) (Class|AnimInstance|IsAnyMontagePlaying (Components|SkeletalMesh|GetAnimInstance (Variables|Default|GetSkeletalMesh))) (!= (Variables|Default|GetMunitionChargeur) 0)))
        (Variables|Default|SetbReloading true)
        (Utilities|FlowControl|Sequence
          (:then_0
            (Animation|Montage|PlayMontage (Variables|Default|GetSkeletalMesh) (Variables|Animation|Weapon|GetMontage%20Reload%20Weapon)
              (:OnCompleted
                (Development|PrintString "Reload Completed")
                ;[1 1 1] Logique Munition
                (if (== (Variables|Default|GetCurrentMunition) 0)
                  (if (>= (Variables|Default|GetMunitionChargeur) (Variables|Default|GetChargeurCapacity))
                    (Variables|Default|SetMunitionChargeur (- (Variables|Default|GetMunitionChargeur) (Variables|Default|GetChargeurCapacity)))
                    (Variables|Default|SetCurrentMunition (Variables|Default|GetChargeurCapacity))
                    (Variables|Default|SetbReloading false)
                    (else
                      (Variables|Default|SetCurrentMunition (Variables|Default|GetMunitionChargeur))
                      (Variables|Default|SetMunitionChargeur 0)
                      (Variables|Default|SetbReloading false)))
                  (else
                    (Variables|Default|SetMunitionChargeur (Math|Integer|Clamp(Integer) (- (Variables|Default|GetMunitionChargeur) (- (Variables|Default|GetChargeurCapacity) (Variables|Default|GetCurrentMunition))) 0 (Variables|Default|GetMunitionMax)))
                    (Variables|Default|SetCurrentMunition (+ (Variables|Default|GetCurrentMunition) (- (Variables|Default|GetChargeurCapacity) (Variables|Default|GetCurrentMunition))))
                    (Variables|Default|SetbReloading false)))
                (Default|CallOnFireUpdate (Variables|/Game/Blueprints/Widget/WBP_Hud.WBP_Hud_C|GetWBP_Weapon (Variables|/Game/Blueprints/BP_FirstPersonPlayerController.BP_FirstPersonPlayerController_C|GetRefHud (Variables|Default|GetAs%20BP%20First%20Person%20Player%20Controller)))))
              (:OnInterrupted
                (Development|PrintString "Weapon Interrupted"))))
          (:then_1
            (Animation|Montage|PlayMontage (Variables|/Game/Blueprints/Characters/Proto/BP_Proto_Player.BP_Proto_Player_C|GetFirstPersonMesh (Variables|Default|GetPlayer)) (Variables|Animation|Arms|GetMontage%20Reload%20Arms)
              (:OnCompleted
                (Variables|/Game/Blueprints/Characters/Proto/BP_Proto_Player.BP_Proto_Player_C|SetbReloading (Variables|Default|GetPlayer) false)))))))
    (:Remote
      (CallFunction|ServerReload))))

(event Custom|Server_Reload
  (CallFunction|StartReload))

(event Custom|Client%20Montage
  (params (MontageToPlay :type Anim%20Montage%20Object%20Reference) (InSkeletalMeshComponent :type Skeletal%20Mesh%20Component%20Object%20Reference))
  (Animation|Montage|PlayMontage InSkeletalMeshComponent MontageToPlay))

(event Custom|Teste%20Animation
  (Animation|Montage|PlayMontage (Variables|Default|GetSkeletalMesh) "/Game/FPS_Pistol_Single/Animations/Pistol/Anim_Pistol_Single_Shot_Montage.Anim_Pistol_Single_Shot_Montage"))

(event EventBeginPlay
  (Variables|Default|SetTimeBetweenShot (/ 6e+01 (Variables|Default|GetRateFire)))
  (bind _asbp_first_person_player_controller (Utilities|Casting|CastToBP_FirstPersonPlayerController (Game|GetInstigatorController (Variables|Default|GetPlayer))))
  (Variables|Default|SetAs%20BP%20First%20Person%20Player%20Controller _asbp_first_person_player_controller)
  (Default|CallOnFireUpdate (Variables|/Game/Blueprints/Widget/WBP_Hud.WBP_Hud_C|GetWBP_Weapon (Variables|/Game/Blueprints/BP_FirstPersonPlayerController.BP_FirstPersonPlayerController_C|GetRefHud (Variables|Default|GetAs%20BP%20First%20Person%20Player%20Controller)))))

(fn ConstructionScript)

(fn StopFire)

(fn StartFire)

(fn CheckMunition
  (return (> (Variables|Default|GetCurrentMunition) 0)))

(fn CheckChargeur
  (return (== (Variables|Default|GetCurrentMunition) (Variables|Default|GetChargeurCapacity))))

(fn CheckMunitionChargeur
  (return (== (Variables|Default|GetMunitionChargeur) 0)))

(fn RefillMunition
  (Variables|Default|SetMunitionChargeur (Variables|Default|GetMunitionMax)))

(fn CheckFullMunition
  (return (== (Variables|Default|GetMunitionChargeur) (Variables|Default|GetMunitionMax))))

(fn SetMunition
  (params (CurrentMunition :type Integer) (MunitionChargeur :type Integer))
  (Variables|Default|SetCurrentMunition CurrentMunition)
  (Variables|Default|SetMunitionChargeur MunitionChargeur))

(fn GetMunition
  (return (Variables|Default|GetCurrentMunition) (Variables|Default|GetMunitionChargeur)))