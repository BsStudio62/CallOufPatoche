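; Prototype hitscan weapon with pistol fire and reload montages, using debug lines, spheres and prints for feedback.
; Fire plays the montage and sets a timer that optionally loops via FireMod, delayed by time since the last shot; StopFire clears it.
; Each shot line-traces from the owner's eyes, adds impulse to simulating components and checks physical surface, sending BPI_Damage only on Head hits.
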(event Custom|Fire
  (bind _returnvalue (Components|GetOwner))
  (bind (_outlocation _outrotation) (Actor|GetActorEyesViewPoint _returnvalue))
  (if (not (Class|KismetSystemLibrary|TimerExistsHandle (Variables|Default|GethandleFire)))
    (bind _returnvalue_2 (Utilities|Time|SetTimerbyEvent (delegate Custom|CustomEvent) (Variables|Default|GetTimeBetweenShot) (Variables|Default|GetFireMod) (Math|Float|Max(Float) (- (+ (Variables|Default|GetLastFireTime) (Variables|Default|GetTimeBetweenShot)) (Utilities|Time|GetTimeSeconds)) 0.0)))
    (Variables|Default|SethandleFire _returnvalue_2)
    (if (not (Variables|Default|GetCurrentFire))
      (Variables|Default|SetCurrentFire false)
      (Animation|Montage|PlayMontage (Variables|Default|GetSkeletalMesh) "/Game/Art/Weapons/Pistol/Animations/Weap_Pistol_Fire_Montage.Weap_Pistol_Fire_Montage"
        (:then
          (bind (_outhit _returnvalue_3) (Collision|LineTraceByChannel _outlocation (+ _outlocation (* (Math|Rotator|GetRotationXVector _outrotation) (Variables|Default|GetDistance))) "TraceTypeQuery1" false (Utilities|Array|MakeArray (Components|GetOwner) self) "None"))
          (Rendering|Debug|DrawDebugLine :LineStart (Transformation|GetSocketLocation (Variables|Default|GetSkeletalMesh) "Muzzle") :LineEnd (Math|Vector|SelectVector (.Location (Collision|BreakHitResult _outhit)) (.TraceEnd (Collision|BreakHitResult _outhit)) _returnvalue_3) :Duration 1.0)
          (Utilities|IsValid (.HitComponent (Collision|BreakHitResult _outhit))
            (:Is%20Valid
              (if (Physics|IsSimulatingPhysics (.HitComponent (Collision|BreakHitResult _outhit)) "None")
                (Physics|AddImpulseatLocation (.HitComponent (Collision|BreakHitResult _outhit)) (* (.ImpactPoint (Collision|BreakHitResult _outhit)) 1e+02) (.Location (Collision|BreakHitResult _outhit)) "None")))
            (:Is%20Not%20Valid
              _))
          (Utilities|IsValid (.PhysMat (Collision|BreakHitResult _outhit))
            (:Is%20Valid
              (Development|PrintString (Utilities|String|EnumtoString (Variables|/Script/PhysicsCore.PhysicalMaterial|GetSurfaceType (.PhysMat (Collision|BreakHitResult _outhit)))))
              (switch Utilities|FlowControl|Switch|SwitchonEPhysicalSurface (Variables|/Script/PhysicsCore.PhysicalMaterial|GetSurfaceType (.PhysMat (Collision|BreakHitResult _outhit)))
                (:SurfaceType_Default
                  (Rendering|Debug|DrawDebugSphere (.Location (Collision|BreakHitResult _outhit)) 1e+01 12 "(R=0.000000,G=1.000000,B=0.096722,A=1.000000)" 0.0)
                  ;[1 1 1] Dernier Tir effectuer
                  (Variables|Default|SetLastFireTime (Utilities|Time|GetTimeSeconds) :!label _label))
                (:SurfaceType1
                  (Rendering|Debug|DrawDebugSphere (.Location (Collision|BreakHitResult _outhit)) 1e+01 12 "(R=1.000000,G=0.000000,B=0.192791,A=1.000000)" 0.0)
                  (Utilities|FlowControl|Sequence
                    (:then_0
                      (goto _label))
                    (:then_1
                      (Utilities|IsValid (.HitActor (Collision|BreakHitResult _outhit))
                        (:Is%20Valid
                          (if (Utilities|DoesObjectImplementInterface (.HitActor (Collision|BreakHitResult _outhit)) "/Game/Blueprints/Interface/BPI_Damage.BPI_Damage_C")
                            (Class|BPIDamage|Damage(Message) (.HitActor (Collision|BreakHitResult _outhit)))))))))))))
        (:OnCompleted
          (Variables|Default|SetCurrentFire false))))))

(event Custom|CustomEvent
  (bind _returnvalue (Components|GetOwner))
  (bind (_outlocation _outrotation) (Actor|GetActorEyesViewPoint _returnvalue))
  (Animation|Montage|PlayMontage (Variables|Default|GetSkeletalMesh) "/Game/Art/Weapons/Pistol/Animations/Weap_Pistol_Fire_Montage.Weap_Pistol_Fire_Montage"
    (:then
      (bind (_outhit _returnvalue_2) (Collision|LineTraceByChannel _outlocation (+ _outlocation (* (Math|Rotator|GetRotationXVector _outrotation) (Variables|Default|GetDistance))) "TraceTypeQuery1" false (Utilities|Array|MakeArray (Components|GetOwner) self) "None"))
      (Rendering|Debug|DrawDebugLine :LineStart (Transformation|GetSocketLocation (Variables|Default|GetSkeletalMesh) "Muzzle") :LineEnd (Math|Vector|SelectVector (.Location (Collision|BreakHitResult _outhit)) (.TraceEnd (Collision|BreakHitResult _outhit)) _returnvalue_2) :Duration 1.0)
      (Utilities|IsValid (.HitComponent (Collision|BreakHitResult _outhit))
        (:Is%20Valid
          (if (Physics|IsSimulatingPhysics (.HitComponent (Collision|BreakHitResult _outhit)) "None")
            (Physics|AddImpulseatLocation (.HitComponent (Collision|BreakHitResult _outhit)) (* (.ImpactPoint (Collision|BreakHitResult _outhit)) 1e+02) (.Location (Collision|BreakHitResult _outhit)) "None")))
        (:Is%20Not%20Valid
          _))
      (Utilities|IsValid (.PhysMat (Collision|BreakHitResult _outhit))
        (:Is%20Valid
          (Development|PrintString (Utilities|String|EnumtoString (Variables|/Script/PhysicsCore.PhysicalMaterial|GetSurfaceType (.PhysMat (Collision|BreakHitResult _outhit)))))
          (switch Utilities|FlowControl|Switch|SwitchonEPhysicalSurface (Variables|/Script/PhysicsCore.PhysicalMaterial|GetSurfaceType (.PhysMat (Collision|BreakHitResult _outhit)))
            (:SurfaceType_Default
              (Rendering|Debug|DrawDebugSphere (.Location (Collision|BreakHitResult _outhit)) 1e+01 12 "(R=0.000000,G=1.000000,B=0.096722,A=1.000000)" 0.0)
              ;[1 1 1] Dernier Tir effectuer
              (Variables|Default|SetLastFireTime (Utilities|Time|GetTimeSeconds) :!label _label))
            (:SurfaceType1
              (Rendering|Debug|DrawDebugSphere (.Location (Collision|BreakHitResult _outhit)) 1e+01 12 "(R=1.000000,G=0.000000,B=0.192791,A=1.000000)" 0.0)
              (Utilities|FlowControl|Sequence
                (:then_0
                  (goto _label))
                (:then_1
                  (Utilities|IsValid (.HitActor (Collision|BreakHitResult _outhit))
                    (:Is%20Valid
                      (if (Utilities|DoesObjectImplementInterface (.HitActor (Collision|BreakHitResult _outhit)) "/Game/Blueprints/Interface/BPI_Damage.BPI_Damage_C")
                        (Class|BPIDamage|Damage(Message) (.HitActor (Collision|BreakHitResult _outhit)))))))))))))
    (:OnCompleted
      (Variables|Default|SetCurrentFire false))))

(event Custom|Stop%20Fire
  (bind _handlefire (Variables|Default|GethandleFire))
  (if (Class|KismetSystemLibrary|TimerExistsHandle _handlefire)
    (Utilities|Time|ClearandInvalidateTimerbyHandle _handlefire)))

(event Custom|Reload
  (Animation|Montage|PlayMontage (Variables|Default|GetSkeletalMesh) "/Game/Art/Weapons/Pistol/Animations/Weap_Pistol_Reload_Montage.Weap_Pistol_Reload_Montage"
    (:OnCompleted
      (Development|PrintString "Reload COmpleted"))))

(event EventBeginPlay
  (Variables|Default|SetTimeBetweenShot 0.67))

(fn ConstructionScript)

(fn StopFire)

(fn StartFire)