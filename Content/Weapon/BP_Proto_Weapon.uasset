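; Prototype hitscan weapon Blueprint with single or automatic fire.
; Fire starts a timer set by FireRate, looping per FireMod, and StopFire clears it.
; Each timer tick line-traces from the owner's eye view, draws a debug line from the muzzle socket, and pushes physics-simulating components with an impulse derived from the impact point.
; Hit physical material surfaces are printed and marked with debug spheres, colouring Head hits differently.
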(event Custom|Fire
  (bind _returnvalue (Utilities|Time|SetTimerbyEvent (delegate Custom|CustomEvent) (/ (Variables|Default|GetFireRate) 6e+01) (Variables|Default|GetFireMod)))
  (Variables|Default|SethandleFire _returnvalue))

(event Custom|CustomEvent
  (bind _returnvalue (Components|GetOwner))
  (bind (_outlocation _outrotation) (Actor|GetActorEyesViewPoint _returnvalue))
  (bind _outhit (Collision|LineTraceByChannel _outlocation (+ _outlocation (* (Math|Rotator|GetRotationXVector _outrotation) (Variables|Default|GetDistance))) "TraceTypeQuery1" false (Utilities|Array|MakeArray (Components|GetOwner) self) "ForDuration"))
  (Rendering|Debug|DrawDebugLine :LineStart (Transformation|GetSocketLocation (Variables|Default|GetSkeletalMesh) "Muzzle") :LineEnd (.TraceEnd (Collision|BreakHitResult _outhit)) :Duration 1.0)
  (Utilities|IsValid (.HitComponent (Collision|BreakHitResult _outhit))
    (:Is%20Valid
      (if (Physics|IsSimulatingPhysics (.HitComponent (Collision|BreakHitResult _outhit)) "None")
        (Physics|AddImpulseatLocation (.HitComponent (Collision|BreakHitResult _outhit)) (* (.ImpactPoint (Collision|BreakHitResult _outhit)) 1e+02) (.Location (Collision|BreakHitResult _outhit)) "None")))
    (:Is%20Not%20Valid
      _))
  (Utilities|IsValid (.PhysMat (Collision|BreakHitResult _outhit))
    (:Is%20Valid
      (Development|PrintString (Utilities|String|EnumtoString (Variables|/Script/PhysicsCore.PhysicalMaterial|GetSurfaceType (.PhysMat (Collision|BreakHitResult _outhit)))))
      (switch Utilities|FlowControl|Switch|SwitchonEPhysicalSurface (Variables|/Script/PhysicsCore.PhysicalMaterial|GetSurfaceType (.PhysMat (Collision|BreakHitResult _outhit)))
        (:SurfaceType_Default
          (Rendering|Debug|DrawDebugSphere (.Location (Collision|BreakHitResult _outhit)) 1e+01 12 "(R=0.000000,G=1.000000,B=0.096722,A=1.000000)" 1.0))
        (:SurfaceType1
          (Rendering|Debug|DrawDebugSphere (.Location (Collision|BreakHitResult _outhit)) 1e+01 12 "(R=1.000000,G=0.000000,B=0.192791,A=1.000000)" 1.0))))))

(event Custom|Stop%20Fire
  (Utilities|Time|ClearandInvalidateTimerbyHandle (Variables|Default|GethandleFire)))

(fn ConstructionScript)